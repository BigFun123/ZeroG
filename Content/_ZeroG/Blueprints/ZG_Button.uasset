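; ZG_Button is a pressure-button actor in the ZeroG game that opens a linked door while something overlaps it.
; Begin overlap sets Down and opens the Door reference, or the Exit reference if no Door is valid.
; End overlap clears Down and closes the Door, or closes the Exit only when AutoClose is enabled.
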(event `self.ReceiveActorBeginOverlap`
  (params (OtherActor :type "Actor Object Reference"))
  (bind _door (`self.Door`))
  (bind _exit (`self.Exit`))
  (set `self.Down` true)
  (`/Engine/EditorBlueprintResources/StandardMacros.IsValid` _door
    (:`Is Valid`
      (`/Game/_ZeroG/Blueprints/ZG_Door.OpenDoor` _door))
    (:`Is Not Valid`
      (`/Engine/EditorBlueprintResources/StandardMacros.IsValid` _exit
        (:`Is Valid`
          (`/Game/_ZeroG/Blueprints/ZG_Exit.OpenDoor` _exit))))))

(event `self.ReceiveActorEndOverlap`
  (params (OtherActor :type "Actor Object Reference"))
  (bind _door (`self.Door`))
  (bind _exit (`self.Exit`))
  (set `self.Down` false)
  (`/Engine/EditorBlueprintResources/StandardMacros.IsValid` _door
    (:`Is Valid`
      (`/Game/_ZeroG/Blueprints/ZG_Door.CloseDoor` _door))
    (:`Is Not Valid`
      (if (`self.AutoClose`)
        (`/Engine/EditorBlueprintResources/StandardMacros.IsValid` _exit
          (:`Is Valid`
            (`/Game/_ZeroG/Blueprints/ZG_Exit.CloseDoor` _exit)))))))

(fn `UserConstructionScript`)