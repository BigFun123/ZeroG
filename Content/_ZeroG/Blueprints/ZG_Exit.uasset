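; ZG_Exit is the level exit actor, with a sliding metal door and an overlap trigger for level progression.
; Any actor overlap calls NextLevel on ZG_GameMode, waits three seconds, then opens a level by name.
; OpenDoor and CloseDoor each stop the opposing timeline, play a door sound and run their own timeline to lerp the door vertically.
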(event `self.ReceiveActorBeginOverlap`
  (params (OtherActor :type "Actor Object Reference"))
  (bind _aszg_game_mode (cast `/Game/_ZeroG/Game/ZG_GameMode` (`GameplayStatics.GetGameMode`)))
  (`/Game/_ZeroG/Game/ZG_GameMode.NextLevel` _aszg_game_mode)
  (`KismetSystemLibrary.Delay` 3.0)
  (`GameplayStatics.GetCurrentLevelName` true)
  (`GameplayStatics.OpenLevel` (`KismetStringLibrary.Conv_StringToName` (`self.Level Name`))))

(event `OpenDoor`
  (bind _door (`self.Door`))
  (`|ExecutionSequence`
    (:`then_0`
      (bind (_direction _closedooranim) (`Timeline|CloseDoor_TL` :!via `Stop` :!label _label)
        (:`Update`
          (`SceneComponent.K2_SetRelativeLocation` _door (`KismetMathLibrary.VLerp` (0.0 0.0 144.0) (0.0 0.0 -158.0) _closedooranim) false false))))
    (:`then_1`
      (`GameplayStatics.PlaySoundAtLocation` "/Game/_ZeroG/Audio/doors/ZGS_Door_Metal.ZGS_Door_Metal" (`self.K2_GetActorLocation`) (struct) 1.0 1.0 0.0 null null null null)
      (bind (_direction_2 _opendooranim) (`Timeline|OpenDoor_TL` :!via `PlayFromStart` :!label _label_2)
        (:`Update`
          (`SceneComponent.K2_SetRelativeLocation` _door (`KismetMathLibrary.VLerp` (0.0 0.0 144.0) (0.0 0.0 -158.0) _opendooranim) false false))))))

(event `CloseDoor`
  (`|ExecutionSequence`
    (:`then_0`
      (goto _label_2 :!via `Stop`))
    (:`then_1`
      (`GameplayStatics.PlaySoundAtLocation` "/Game/_ZeroG/Audio/doors/ZGS_Door_Metal_Close.ZGS_Door_Metal_Close" (`self.K2_GetActorLocation`) (struct) 1.0 1.0 0.0 null null null null)
      (goto _label :!via `PlayFromStart`))))

(fn `UserConstructionScript`)