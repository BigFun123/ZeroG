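; ZG_Door is a Blueprint for a sliding metal door, driven by OpenDoor and CloseDoor events.
; OpenDoor plays a sound and runs a timeline that lerps the door's relative position downward, setting Open when it finishes.
; CloseDoor plays its own sound, clears Open, snaps the door straight back to its raised position and stops the timeline, so closing is not animated.
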(event `OpenDoor`
  (`GameplayStatics.PlaySoundAtLocation` "/Game/_ZeroG/Audio/doors/ZGS_Door_Metal.ZGS_Door_Metal" (`self.K2_GetActorLocation`) (struct) 1.0 1.0 0.0 null null null null)
  (bind (_direction _opentrack) (`Timeline|OpenDoorTimeline` :!via `PlayFromStart` :!label _label)
    (:`Update`
      (`SceneComponent.K2_SetRelativeLocation` (`self.door`) (`KismetMathLibrary.VLerp` (0.0 0.0 150.0) (0.0 0.0 -150.0) _opentrack) false false))
    (:`Finished`
      (set `self.Open` true))))

(event `CloseDoor`
  (`GameplayStatics.PlaySoundAtLocation` "/Game/_ZeroG/Audio/doors/ZGS_Door_Metal_Close.ZGS_Door_Metal_Close" (`self.K2_GetActorLocation`) (struct) 1.0 1.0 0.0 null null null null)
  (set `self.Open` false)
  (`SceneComponent.K2_SetRelativeLocation` (`self.door`) (0.0 0.0 150.0) false false)
  (goto _label :!via `Stop`))

(fn `UserConstructionScript`)